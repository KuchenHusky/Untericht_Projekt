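; BP_PressurPlate is a pressure plate that switches linked actors on and off when Characters step on or off it.
; A timeline lowers the plate top on box overlap and reverses on exit unless OneWay is set.
; When the animation finishes, it sends the on/off state to TriggerTargets via BPI_Trigger, and the first press also plays an optional LevelSequence.
; Any overlap plays a sound at world origin, before the Character check.
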(event `self.ReceiveBeginPlay`
  (`TimelineComponent.SetPlayRate` (`self.ButtonAnim`) 5.0))

(event `self.BoxCollision.OnComponentBeginOverlap`
  (params (OverlappedComponent :type "PrimitiveComponent Object Reference") (OtherActor :type "Actor Object Reference") (OtherComp :type "PrimitiveComponent Object Reference") (OtherBodyIndex :type Integer) (bFromSweep :type Boolean) (SweepResult :type "HitResult Structure (by ref)"))
  (bind _levelsequence (`self.LevelSequence`))
  (`GameplayStatics.PlaySoundAtLocation` "/Game/Audio/Sounds/PresureplateSounds/MS_Presureplate.MS_Presureplate" (0.0 0.0 0.0) (struct) 1.0 1.0 0.0 null null null null)
  (cast `Character` OtherActor)
  (bind (_direction _alpha) (`Timeline|ButtonAnim` :!label _label)
    (:`Update`
      (`SceneComponent.K2_SetRelativeLocation` (`self.SM_PressurPlateTop`) (`KismetMathLibrary.VLerp` (0.0 0.0 0.0) (0.0 0.0 -7.0) _alpha) false false))
    (:`Finished`
      (switch `ETimelineDirection` _direction
        (:`Forward`
          (`|ExecutionSequence`
            (:`then_0`
              (`/Engine/EditorBlueprintResources/StandardMacros.DoOnce` false
                (:`Completed`
                  ;[1 1 1] LevelSequence
                  (`/Engine/EditorBlueprintResources/StandardMacros.IsValid` _levelsequence
                    (:`Is Valid`
                      (`MovieSceneSequencePlayer.Play` (`LevelSequenceActor.SequencePlayer` _levelsequence)))))))
            (:`then_1`
              (set `self.IsOn` true)
              ;[1 1 1] Triggerable Actors | On
              (for _array_element (`self.TriggerTargets`) :!label _label_2
                (if (`KismetSystemLibrary.DoesImplementInterface` _array_element "/Game/Blueprints/Interfaces/BPI_Trigger.BPI_Trigger_C")
                  (message `/Game/Blueprints/Interfaces/BPI_Trigger.Trigger` _array_element (`self.IsOn`) null))))))
        (:`Backward`
          (set `self.IsOn` false)
          (goto _label_2))))))

(event `self.BoxCollision.OnComponentEndOverlap`
  (params (OverlappedComponent :type "PrimitiveComponent Object Reference") (OtherActor :type "Actor Object Reference") (OtherComp :type "PrimitiveComponent Object Reference") (OtherBodyIndex :type Integer))
  (cast `Character` OtherActor)
  (if (not (`self.OneWay`))
    (goto _label :!via `Reverse`)))

(fn `UserConstructionScript`)