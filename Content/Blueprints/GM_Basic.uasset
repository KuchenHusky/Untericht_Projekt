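; GM_Basic is a basic game mode that handles player spawning, score, game UI and pausing.
; On BeginPlay it records the placed BP_Player's transform as the spawnpoint and creates WBP_GameUI with a gameplay layer.
; PlayerSpawn spawns and possesses a new player at that point, while AddScore updates the score and UI.
; Pause and unpause manage a separate widget stack, game pause, input mode and mouse cursor.
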(event `self.ReceiveBeginPlay`
  (`self.Setup Spawnpoint`)
  (`self.Setup UI`))

(event `Setup Spawnpoint`
  (bind _returnvalue (`GameplayStatics.GetActorOfClass` "/Game/Blueprints/BP_Player.BP_Player_C"))
  (set `self.PlayerSpawnpoint` (`self.GetTransform` _returnvalue)))

(event `PlayerSpawn`
  (bind (_playerspawnpoint_location _playerspawnpoint_rotation) (`KismetMathLibrary.BreakTransform` (`self.PlayerSpawnpoint`)))
  ;[1 1 1] Comment
  (bind _returnvalue (`|SpawnActorFromClass` "/Game/Blueprints/BP_Player.BP_Player_C" (`KismetMathLibrary.MakeTransform` _playerspawnpoint_location _playerspawnpoint_rotation) "Undefined" "MultiplyWithRoot" null null))
  (`Controller.Possess` (`GameplayStatics.GetPlayerController` 0) _returnvalue))

(event `AddScore`
  (params (Value :type Integer))
  ;[1 1 1] ScoreText
  (bind _output_get (set `self.Score` (+ Value (`self.Score`))))
  (`/Game/UI/WBP_GameUI.UpdateScore` (`self.GameUI`) _output_get))

(event `Setup UI`
  ;[1 1 1] Setup UI
  (bind _returnvalue (`|CreateWidget` "/Game/UI/WBP_GameUI.WBP_GameUI_C"))
  (bind _output_get (set `self.GameUI` _returnvalue))
  (`UserWidget.AddToViewport` _output_get 0)
  (`CommonActivatableWidgetContainerBase.BP_AddWidget` (`/Game/UI/WBP_GameUI.GameplayStack` _output_get) "/Game/UI/WBP_GameplayUI.WBP_GameplayUI_C"))

(event `Pause Game`
  (bind _returnvalue (`GameplayStatics.GetPlayerController` 0))
  (`CommonActivatableWidgetContainerBase.BP_AddWidget` (`/Game/UI/WBP_GameUI.PauseStack` (`self.GameUI`)) "/Game/UI/WBP_PausMenuBase.WBP_PausMenuBase_C")
  (`GameplayStatics.SetGamePaused` true)
  (`WidgetBlueprintLibrary.SetInputMode_UIOnlyEx` _returnvalue null)
  (set `PlayerController.bShowMouseCursor` true _returnvalue))

(event `Unpause Game`
  (bind _returnvalue (`GameplayStatics.GetPlayerController` 0))
  (`CommonActivatableWidgetContainerBase.ClearWidgets` (`/Game/UI/WBP_GameUI.PauseStack` (`self.GameUI`)))
  (`GameplayStatics.SetGamePaused` false)
  (`WidgetBlueprintLibrary.SetInputMode_GameOnly` _returnvalue)
  (set `PlayerController.bShowMouseCursor` false _returnvalue))

(fn `UserConstructionScript`)