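; BP_FallingPlatform is a platform that disappears after a Character overlaps its Box, then respawns.
; A DoOnce gate starts the cycle: a delay, removal, a second delay, then restoration.
; The ScaleAnim timeline drives uniform actor scale, disabling collision and hiding the actor when forward play finishes.
; Restoration re-enables collision and visibility, resets the gate, and reverses the timeline.
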(event `self.Box.OnComponentBeginOverlap`
  (params (OverlappedComponent :type "PrimitiveComponent Object Reference") (OtherActor :type "Actor Object Reference") (OtherComp :type "PrimitiveComponent Object Reference") (OtherBodyIndex :type Integer) (bFromSweep :type Boolean) (SweepResult :type "HitResult Structure (by ref)"))
  (cast `Character` OtherActor)
  (`/Engine/EditorBlueprintResources/StandardMacros.DoOnce` false :!label _label
    (:`Completed`
      (`KismetSystemLibrary.Delay` (`self.Delay until Triggerd`))
      (`self.Animate Platform` false)
      (`KismetSystemLibrary.Delay` (`self.Delay Until Respawn`))
      (`self.Animate Platform` true))))

(event `Reset`
  (goto _label :!via `Reset`))

(event `Animate Platform`
  (params (Visible :type Boolean))
  (if (not Visible)
    (bind (_direction _alpha) (`Timeline|ScaleAnim` :!label _label_2)
      (:`Update`
        (`self.SetActorScale3D` (`KismetMathLibrary.Conv_DoubleToVector` _alpha)))
      (:`Finished`
        (switch `ETimelineDirection` _direction
          (:`Forward`
            (`self.Toogle Collision` false)))))
    (else
      (`self.Toogle Collision` true)
      (`self.Reset`)
      (goto _label_2 :!via `Reverse`))))

(event `Toogle Collision`
  (params (Enable :type Boolean))
  (`self.SetActorEnableCollision` Enable)
  (`self.SetActorHiddenInGame` (not Enable)))

(fn `UserConstructionScript`)